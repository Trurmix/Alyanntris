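; Door Blueprint that the player can toggle open and closed when close to it.
; Box overlap events set a DoUEvenDoor proximity flag that gates the MyDoorOpen event.
; A FlipFlop alternates between playing and reversing the RotationDoor timeline, whose DoorRot track drives the Door's relative yaw.
; The overlap events do not filter which actor enters or leaves the box.
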(event OnComponentBeginOverlap(Box)
  (params (OverlappedComponent :type Primitive%20Component%20Object%20Reference) (OtherActor :type Actor%20Object%20Reference) (OtherComp :type Primitive%20Component%20Object%20Reference) (OtherBodyIndex :type Integer) (bFromSweep :type Boolean) (SweepResult :type Hit%20Result%20Structure%20%28by%20ref%29))
  ;[1 1 1] Close to the door
  (Variables|Default|SetDoUEvenDoor? true))

(event OnComponentEndOverlap(Box)
  (params (OverlappedComponent :type Primitive%20Component%20Object%20Reference) (OtherActor :type Actor%20Object%20Reference) (OtherComp :type Primitive%20Component%20Object%20Reference) (OtherBodyIndex :type Integer))
  ;[1 1 1] Close to the door
  (Variables|Default|SetDoUEvenDoor? false))

(event Custom|MyDoorOpen
  ;[1 1 1] Open Dooooooor
  (if (Variables|Default|GetDoUEvenDoor?)
    (Utilities|FlowControl|FlipFlop
      (:A
        (bind _doorrot (Timeline|RotationDoor Play)
          (:Update
            (Transformation|SetRelativeRotation (Variables|Default|GetDoor) (Math|Rotator|MakeRotator 0.0 0.0 _doorrot) false false))))
      (:B
        (Timeline|RotationDoor Reverse)))))

(fn ConstructionScript)