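; BP_BadSoul-1 is an overlap pickup that raises the BadSouls value on the -1Character that touches it.
; On overlap it calls a fade-in and then immediately a fade-out on its AudioCurveSource.
; Unless BadSouls already exceeds its cap, it adds a fixed increment, clamps the result to that cap and destroys itself.
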(event Collision|EventActorBeginOverlap
  (params (OtherActor :type Actor%20Object%20Reference))
  (bind _as__1character (Utilities|Casting|CastTo-1Character OtherActor))
  (Audio|Components|Audio|FadeIn (Variables|Default|GetAudioCurveSource) 1e+01 1.0 0.0 :!class /Script/Engine.AudioComponent)
  (Audio|Components|Audio|FadeOut (Variables|Default|GetAudioCurveSource) 1e+01 0.5 :!class /Script/Engine.AudioComponent)
  (if (not (> (Variables|/Game/Floors/-1/-1Character.-1Character_C|GetBadSouls _as__1character) 1.0))
    (bind _output_get (Variables|/Game/Floors/-1/-1Character.-1Character_C|SetBadSouls _as__1character (+ (Variables|/Game/Floors/-1/-1Character.-1Character_C|GetBadSouls _as__1character) 0.11)))
    (if (> _output_get 1.0)
      (Variables|/Game/Floors/-1/-1Character.-1Character_C|SetBadSouls _as__1character 1.0))
    (Actor|DestroyActor)))

(fn ConstructionScript)